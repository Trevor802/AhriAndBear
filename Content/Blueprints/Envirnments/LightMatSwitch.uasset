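; Environment actor that makes the light meshes in LightActor glow or go dark to match a linked TargetLightSwitch.
; It applies the switch state on BeginPlay, then polls CurrentOn every Tick and reacts only when it differs from the stored previous state.
; On each change, it creates a dynamic material instance on each mesh's LightIndex slot and sets Illum_Intensity to IlluminateIntensity or zero.
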(event `self.ReceiveBeginPlay`
  (bind _bcurrenton (`LightSwitchInteractive.bCurrentOn` (`self.Target Light Switch`)))
  (`|ExecutionSequence`
    (:`then_0`
      (if _bcurrenton
        (`self.Show Material Light`)
        (else
          (`self.Hide Material Light`))))
    (:`then_1`
      (set `self.Light Previous State` _bcurrenton))))

(event `self.ReceiveTick`
  (params (DeltaSeconds :type "Float (single-precision)"))
  (bind _bcurrenton (`LightSwitchInteractive.bCurrentOn` (`self.Target Light Switch`)))
  (if (!= _bcurrenton (`self.Light Previous State`))
    (`|ExecutionSequence`
      (:`then_0`
        (if _bcurrenton
          (`self.Show Material Light`)
          (else
            (`self.Hide Material Light`))))
      (:`then_1`
        (set `self.Light Previous State` _bcurrenton)))))

(event `Show Material Light`
  (bind _light_index (`self.Light Index`))
  (for _array_element (`self.Light Actor`)
    (bind _returnvalue (`self.GetComponentByClass` _array_element "/Script/Engine.StaticMeshComponent"))
    (bind _returnvalue_2 (`PrimitiveComponent.CreateDynamicMaterialInstance` _returnvalue _light_index (`PrimitiveComponent.GetMaterial` _returnvalue _light_index) "None"))
    (`MaterialInstanceDynamic.SetScalarParameterValue` _returnvalue_2 "Illum_Intensity" (`self.Illuminate Intensity`))))

(event `Hide Material Light`
  (bind _light_index (`self.Light Index`))
  (for _array_element (`self.Light Actor`)
    (bind _returnvalue (`self.GetComponentByClass` _array_element "/Script/Engine.StaticMeshComponent"))
    (bind _returnvalue_2 (`PrimitiveComponent.CreateDynamicMaterialInstance` _returnvalue _light_index (`PrimitiveComponent.GetMaterial` _returnvalue _light_index) "None"))
    (`MaterialInstanceDynamic.SetScalarParameterValue` _returnvalue_2 "Illum_Intensity" 0.0)))

(fn `UserConstructionScript`)