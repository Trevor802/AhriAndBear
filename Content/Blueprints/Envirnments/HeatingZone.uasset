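; HeatingZone is an overlap volume that changes the warmth change speed of cat and dog characters inside it.
; On entry it saves each character's speed and applies WarmSpeed; on exit it restores the saved value.
; VFX activation and deactivation run only on the dog branch, with shutoff once both saved speeds are zero.
; The sound call on dog entry is an unfinished TODO at world origin.
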(event `self.ReceiveActorBeginOverlap`
  (params (OtherActor :type "Actor Object Reference"))
  ;[1 1 1] Set cat warmth change speed
  (bind _asbp_cat_character (cast `/Game/Blueprints/GameMode/BP_CatCharacter` OtherActor)
    (:`then`
      (set `self.PrevCatWarm` (`/Game/Blueprints/GameMode/BP_AnimalCharacter.WarmthChangeSpeed` _asbp_cat_character))
      (set `/Game/Blueprints/GameMode/BP_AnimalCharacter.WarmthChangeSpeed` (`self.WarmSpeed`) _asbp_cat_character)
      (set `self.IsHeating` true))
    (:`CastFailed`
      _))
  ;[1 1 1] Set dog warmth change speed
  (bind _asbp_dog_character (cast `/Game/Blueprints/GameMode/BP_DogCharacter` OtherActor))
  (set `self.PrevDogWarm` (`/Game/Blueprints/GameMode/BP_AnimalCharacter.WarmthChangeSpeed` _asbp_dog_character))
  (set `/Game/Blueprints/GameMode/BP_AnimalCharacter.WarmthChangeSpeed` (`self.WarmSpeed`) _asbp_dog_character)
  (set `self.IsHeating` true)
  (`ActorComponent.Activate` (`self.VFX`) false)
  ;[1 1 1] TODO
  (`GameplayStatics.PlaySoundAtLocation` null (0.0 0.0 0.0) (struct) 1.0 1.0 0.0 null null null))

(event `self.ReceiveActorEndOverlap`
  (params (OtherActor :type "Actor Object Reference"))
  (bind _asbp_cat_character (cast `/Game/Blueprints/GameMode/BP_CatCharacter` OtherActor)
    (:`then`
      (set `/Game/Blueprints/GameMode/BP_AnimalCharacter.WarmthChangeSpeed` (`self.PrevCatWarm`) _asbp_cat_character)
      (set `self.PrevCatWarm` 0.0))
    (:`CastFailed`
      _))
  (bind _asbp_dog_character (cast `/Game/Blueprints/GameMode/BP_DogCharacter` OtherActor))
  (set `/Game/Blueprints/GameMode/BP_AnimalCharacter.WarmthChangeSpeed` (`self.PrevDogWarm`) _asbp_dog_character)
  (set `self.PrevDogWarm` 0.0)
  (if (and (== (`self.PrevCatWarm`) 0.0) (== (`self.PrevDogWarm`) 0.0))
    (set `self.IsHeating` false)
    (`ActorComponent.Deactivate` (`self.VFX`))))

(fn `UserConstructionScript`)