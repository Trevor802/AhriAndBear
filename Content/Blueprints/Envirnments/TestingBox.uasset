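; TestingBox is an actor with a static mesh that an ABAnimalCharacter pushes by overlapping it.
; Begin and end overlap events toggle a Pushing flag, and begin overlap also stores the character reference.
; While Pushing is set, Tick applies a force to the mesh along the character root component's forward vector, scaled by the mesh's mass.
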(event `self.ReceiveActorEndOverlap`
  (params (OtherActor :type "Actor Object Reference"))
  (cast `ABAnimalCharacter` OtherActor)
  (set `self.Pushing` false))

(event `self.ReceiveActorBeginOverlap`
  (params (OtherActor :type "Actor Object Reference"))
  (bind _asabanimal_character (cast `ABAnimalCharacter` OtherActor))
  (set `self.Pushing` true)
  (set `self.CharacterRef` _asabanimal_character))

(event `self.ReceiveTick`
  (params (DeltaSeconds :type "Float (single-precision)"))
  (if (`self.Pushing`)
    (`PrimitiveComponent.AddForce` (`self.StaticMesh`) (* (`SceneComponent.GetForwardVector` (`Actor.RootComponent` (`self.CharacterRef`))) (* (`PrimitiveComponent.GetMass` (`self.StaticMesh`)) 1000.0)) "None" false)))

(fn `UserConstructionScript`)