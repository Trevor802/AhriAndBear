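; ScentLine is a Blueprint that lays a hidden scent trail along a spline and reveals it on a show-scent-trail event.
; On BeginPlay, InitTrail spawns deactivated NS_smell systems at regular intervals along the spline, each randomly jittered within a small box, and stores them in ScentUnits.
; The bound event calls ShowTrail to activate these pre-spawned systems.
; HideTrail deactivates them but is not called within this Blueprint.
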(event `self.ReceiveBeginPlay`
  (`self.InitTrail`)
  (add `self.ShowScentTrail` (delegate `Show`)))

(event `Show`
  (`self.ShowTrail`))

(fn `HideTrail`
  (for _array_element (`self.ScentUnits`)
    (`ActorComponent.Deactivate` _array_element)))

(fn `InitTrail`
  (bind _returnvalue (`KismetMathLibrary.Conv_IntToDouble` (`self.Interval`)))
  (for _index (range (+ (`KismetMathLibrary.FTrunc` (/ (`SplineComponent.GetSplineLength` (`self.Spline`)) _returnvalue)) 1))
    (bind _returnvalue_2 (`NiagaraFunctionLibrary.SpawnSystemAtLocation` "/Game/Assets/VFX/NS_smell.NS_smell" (`KismetMathLibrary.RandomPointInBoundingBox` (`SplineComponent.GetLocationAtDistanceAlongSpline` (`self.Spline`) (* _index _returnvalue) "World") (10.0 10.0 10.0)) (struct) false))
    (`ActorComponent.Deactivate` _returnvalue_2)
    (`KismetArrayLibrary.Array_Add` (`self.ScentUnits`) _returnvalue_2)))

(fn `ShowTrail`
  (for _array_element (`self.ScentUnits`)
    (`ActorComponent.Activate` _array_element false)))

(fn `UserConstructionScript`)