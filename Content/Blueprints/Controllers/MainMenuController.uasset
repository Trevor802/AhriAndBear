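; Main menu controller that routes UI input to the menu's MainMenuButton object.
; It caches that reference from the HUD_MainMenu actor on BeginPlay, and each input event re-fetches it if it has become invalid.
; Selection and slider axes drive vertical and horizontal selection changes, with the vertical value inverted, while confirm and cancel presses are forwarded directly.
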(event `self.ReceiveBeginPlay`
  (bind _returnvalue (`GameplayStatics.GetActorOfClass` "/Game/Blueprints/UI/HUD_MainMenu.HUD_MainMenu_C"))
  (set `self.Main Menu Button` (`/Game/Blueprints/UI/HUD_MainMenu.Main Menu Button` _returnvalue)))

(event `InputAxis|UI_SelectionChange` :consume false :paused true
  (params (AxisValue :type "Float (single-precision)"))
  (`self.Validate Main Menu Button`)
  (`GamepadCompatibleWidget.UIVerticalSelectionChanged` (`self.Main Menu Button`) (* AxisValue -1.0)))

(event `InputAction|UI_Confirm` :consume false :paused true
  (params (Key :type "Key Structure"))
  (:`Pressed`
    (`self.Validate Main Menu Button`)
    (`GamepadCompatibleWidget.UIConfirmPressed` (`self.Main Menu Button`))))

(event `InputAction|UI_Cancel` :consume false :paused true
  (params (Key :type "Key Structure"))
  (:`Pressed`
    (`self.Validate Main Menu Button`)
    (`GamepadCompatibleWidget.UICancelPressed` (`self.Main Menu Button`))))

(event `InputAxis|UI_SliderChange` :consume false :paused true
  (params (AxisValue :type "Float (single-precision)"))
  (`self.Validate Main Menu Button`)
  (`GamepadCompatibleWidget.UIHorizontalSelectionChanged` (`self.Main Menu Button`) AxisValue))

(fn `UserConstructionScript`)

(fn `Validate Main Menu Button`
  (`/Engine/EditorBlueprintResources/StandardMacros.IsValid` (`self.Main Menu Button`)
    (:`Is Not Valid`
      (bind _returnvalue (`GameplayStatics.GetActorOfClass` "/Game/Blueprints/UI/HUD_MainMenu.HUD_MainMenu_C"))
      (set `self.Main Menu Button` (`/Game/Blueprints/UI/HUD_MainMenu.Main Menu Button` _returnvalue)))))