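; DevTools is a debug helper actor that teleports the dog and cat characters to preset warp points through keyboard shortcuts.
; It caches both characters on BeginPlay and tracks either-side Ctrl and Alt state for the KeyComboDown check that gates the number keys 1–4.
; WarpAnimals bounds-checks the WarpPoints index, then moves each animal to its own location actor, printing a message if that actor is invalid.
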(event `self.ReceiveBeginPlay`
  (bind _returnvalue (`GameplayStatics.GetActorOfClass` "/Script/AhriAndBear.ABDogCharacter"))
  (set `self.Dog` _returnvalue)
  (bind _returnvalue_2 (`GameplayStatics.GetActorOfClass` "/Script/AhriAndBear.ABCatCharacter"))
  (set `self.Cat` _returnvalue_2))

(event `Key|LeftControl`
  (params (Key :type "Key Structure"))
  (:`Pressed`
    (set `self.CtrlDown` true :!label _label))
  (:`Released`
    (set `self.CtrlDown` false :!label _label_2)))

(event `Key|One`
  (params (Key :type "Key Structure"))
  (:`Pressed`
    (if (`self.KeyComboDown`)
      (`self.Warp Animals` 0))))

(event `Key|RightControl`
  (params (Key :type "Key Structure"))
  (:`Pressed`
    (goto _label))
  (:`Released`
    (goto _label_2)))

(event `Key|Two`
  (params (Key :type "Key Structure"))
  (:`Pressed`
    (if (`self.KeyComboDown`)
      (`self.Warp Animals` 1))))

(event `Key|LeftAlt`
  (params (Key :type "Key Structure"))
  (:`Pressed`
    (set `self.AltDown` true :!label _label_3))
  (:`Released`
    (set `self.AltDown` false :!label _label_4)))

(event `Key|Three`
  (params (Key :type "Key Structure"))
  (:`Pressed`
    (if (`self.KeyComboDown`)
      (`self.Warp Animals` 2))))

(event `Key|RightAlt`
  (params (Key :type "Key Structure"))
  (:`Pressed`
    (goto _label_3))
  (:`Released`
    (goto _label_4)))

(event `Key|Four`
  (params (Key :type "Key Structure"))
  (:`Pressed`
    (if (`self.KeyComboDown`)
      (`self.Warp Animals` 3))))

(fn `UserConstructionScript`)

(fn `Warp Animals`
  (params (`Warp Point` :type Integer))
  (bind _warp_points (`self.Warp Points`))
  (bind (_output_warppointname _output_dogwarplocation _output_catwarplocation) (break `/Game/Blueprints/Controllers/DevWarpPoint` (`|GetArrayItem` _warp_points `Warp Point`)))
  (if (< `Warp Point` (`KismetArrayLibrary.Array_Length` _warp_points))
    (`|ExecutionSequence`
      (:`then_0`
        (`/Engine/EditorBlueprintResources/StandardMacros.IsValid` _output_dogwarplocation
          (:`Is Valid`
            (`self.K2_SetActorLocation` (`self.Dog`) (`self.K2_GetActorLocation` _output_dogwarplocation) false false))
          (:`Is Not Valid`
            (`KismetSystemLibrary.PrintString` "Dog Warp Location is invalid"))))
      (:`then_1`
        (`/Engine/EditorBlueprintResources/StandardMacros.IsValid` _output_catwarplocation
          (:`Is Valid`
            (`self.K2_SetActorLocation` (`self.Cat`) (`self.K2_GetActorLocation` _output_catwarplocation) false false))
          (:`Is Not Valid`
            (`KismetSystemLibrary.PrintString` "Cat Warp Location is invalid")))))))