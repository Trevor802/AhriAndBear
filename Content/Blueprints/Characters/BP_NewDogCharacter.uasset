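; Dog player character that pants while sprinting, emits AI noise and can carry the cat.
; Sprint start and end events drive a looping timer that replays the panting sound at clip-length intervals, while SprintUpdate reports noise.
; Combine input checks distance and line of sight, then unpossesses the cat and attaches it to the dog.
; Pressing again or switching characters detaches the cat and restores its controller.
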(event `Play Sprint Noise`
  (bind _returnvalue (`GameplayStatics.SpawnSound2D` (`self.Sprinting Sound Clip`) 1.0 1.0 0.0 null))
  (set `self.Sprinting Audio` _returnvalue))

(event `Start Dog Panting`
  (bind _duration (`SoundBase.Duration` (`self.Sprinting Sound Clip`)))
  (bind _returnvalue (`KismetSystemLibrary.K2_SetTimerDelegate` (delegate `Play Sprint Noise`) _duration true (- 0.0 _duration)))
  (set `self.Sprint Sound Off Timer` _returnvalue))

(event `self.ReceiveBeginPlay`
  (set `NavMovementComponent.NavAgentProps` (make `NavAgentProperties` 31.0 47.0 -1.0 0.5 "None" false true true) (`self.CharacterMovement`))
  (add `self.OnSprintStart` (delegate `Start Dog Panting`))
  (add `self.OnSprintEnd` (delegate `Stop Dog Panting`)))

(event `Stop Dog Panting`
  (`KismetSystemLibrary.K2_ClearAndInvalidateTimerHandle` (`self.Sprint Sound Off Timer`))
  (`AudioComponent.Stop` (`self.Sprinting Audio`)))

(event `self.SprintUpdate`
  (`self.MakeNoise` 1.0 null (`self.K2_GetActorLocation`) 0.0 "Noise Event"))

(event `InputAction|AnimalCombine`
  (params (Key :type "Key Structure"))
  (:`Pressed`
    (`self.Character Combination` false)))

(event `self.BeforeCharacterSwitch`
  (`self.Character Combination` true))

(fn `Can Animals Combine`
  (params (Actor :type "Actor Object Reference"))
  (returns (Success :type Boolean))
  (bind _returnvalue (`self.K2_GetActorLocation`))
  (bind _returnvalue_2 (`self.K2_GetActorLocation` Actor))
  (if (<= (`KismetMathLibrary.Vector_Distance` _returnvalue _returnvalue_2) (`self.Distance Before Combination`))
    (bind (_outhit _returnvalue_3) (`KismetSystemLibrary.LineTraceSingle` _returnvalue _returnvalue_2 "TraceTypeQuery1" true))
    (if _returnvalue_3
      (cast `ABCatCharacter` (`.HitActor` (`GameplayStatics.BreakHitResult` _outhit))
        (:`then`
          (return true))
        (:`CastFailed`
          _)))
    (return false)
    (else
      (return false))))

(fn `Character Combination`
  (params (`Force Detach` :type Boolean))
  (bind _otheranimal (`self.OtherAnimal`))
  (bind _returnvalue (`self.GetController` (`self.OtherAnimal`)))
  (if `Force Detach`
    (if (`self.AnimalsCombined`) :!label _label
      (cast `ABCatCharacter` _otheranimal)
      (`self.K2_DetachFromActor` _otheranimal "KeepWorld" "KeepWorld" "KeepWorld")
      (`Controller.Possess` (`self.Other Controller`) (`self.OtherAnimal`))
      (set `self.AnimalsCombined` false))
    (elif (`self.AnimalsCombined`)
      (goto _label)
      (elif (`self.Can Animals Combine` (`self.OtherAnimal`))
        (set `self.Other Controller` _returnvalue)
        (`Controller.UnPossess` _returnvalue)
        (`self.K2_AttachToComponent` (`self.OtherAnimal`) (`self.Animal Combine Point`) "None" "SnapToTarget" "SnapToTarget" "KeepWorld" false)
        (set `self.AnimalsCombined` true)))))

(fn `UserConstructionScript`)