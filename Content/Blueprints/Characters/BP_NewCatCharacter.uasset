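; BP_NewCatCharacter is a cat character Blueprint that shows a stamina bar beside the cat while it is the player character.
; On BeginPlay it creates a CatStaminaStateBar widget, adds it to the viewport and passes itself in as the Cat reference.
; Each tick it projects the cat's location plus WidgetOffset to screen space to position the bar, hiding it when the cat is not player character 0.
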(event `self.ReceiveBeginPlay`
  (bind _returnvalue (`|CreateWidget` "/Game/Blueprints/Widget/StateBar/CatStaminaStateBar.CatStaminaStateBar_C"))
  (`UserWidget.AddToViewport` _returnvalue 0)
  (set `/Game/Blueprints/Widget/StateBar/CatStaminaStateBar.Cat` self _returnvalue)
  (set `self.Stamina Bar` _returnvalue))

(event `self.ReceiveTick`
  (params (DeltaSeconds :type "Float (single-precision)"))
  (if (== (`GameplayStatics.GetPlayerCharacter` 0) self)
    (`UserWidget.SetPositionInViewport` (`self.Stamina Bar`) (`PlayerController.ProjectWorldLocationToScreen` (`GameplayStatics.GetPlayerController` 0) (+ (`self.K2_GetActorLocation`) (`self.Widget Offset`)) false) true)
    (`Widget.SetVisibility` (`self.Stamina Bar`) "Visible")
    (else
      (`Widget.SetVisibility` (`self.Stamina Bar`) "Hidden"))))

(fn `UserConstructionScript`)