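; Bobby enemy character that detects and catches animal characters, with patrol point lookup and print-only melee and ranged attack stubs.
; AI perception sight starts a timed detection that drives a meter widget, while tagged noises briefly flag the heard location.
; Detection requires players inside BP_PlayerInRange; once detected, Tick tracks target position and proximity.
; The distance-based detection multiplier compares Bobby's location with itself, so distance is always zero.
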(event `self.ReceiveBeginPlay`
  (`|ExecutionSequence`
    (:`then_0`
      (bind _asbp_bobby_controller (cast `/Game/Blueprints/AI/Bobby/BP_BobbyController` (`self.GetController`)))
      (add `AIPerceptionComponent.OnTargetPerceptionUpdated` (`/Game/Blueprints/AI/Bobby/BP_BobbyController.AIPerception` _asbp_bobby_controller) (delegate `OnTargetPerceptionUpdated_Event`))
      (bind _asumg_detection_meter (cast `/Game/Blueprints/Widget/Enemies/UMG_DetectionMeter` (`WidgetComponent.GetUserWidgetObject` (`self.Detection Meter`))))
      (set `/Game/Blueprints/Widget/Enemies/UMG_DetectionMeter.Bobby Enemy` self _asumg_detection_meter))
    (:`then_1`
      (bind _returnvalue (`GameplayStatics.GetActorOfClass` "/Game/Blueprints/AI/BP_PlayerInRange.BP_PlayerInRange_C"))
      (set `self.Player In Range` _returnvalue))))

(event `OnTargetPerceptionUpdated_Event`
  (params (Actor :type "Actor Object Reference") (Stimulus :type "AIStimulus Structure"))
  (bind (_age _expirationage _strength _stimuluslocation _receiverlocation _tag _bsuccessfullysensed) (break `AIStimulus` Stimulus))
  (bind _returnvalue (and _bsuccessfullysensed (> (`/Game/Blueprints/AI/BP_PlayerInRange.Total Players Inside` (`self.Player In Range`)) 0)))
  (`|ExecutionSequence`
    (:`then_0`
      (bind _returnvalue_2 (`AIPerceptionSystem.GetSenseClassForStimulus` Stimulus))
      (if (== _returnvalue_2 "/Script/AIModule.AISense_Sight")
        (bind _asabanimal_character (cast `ABAnimalCharacter` Actor))
        (set `self.Current Animal Actor` _asabanimal_character)
        (bind _output_get (set `self.Is Enemy Detecting` _returnvalue))
        (if (not _output_get)
          (set `self.Is Player Detected` false)
          (set `self.Current Detection Time` 0.0))))
    (:`then_1`
      (if _returnvalue
        (if (== _tag (`self.Noise Event`))
          (set `self.Enemy Audio Notified` true)
          (set `self.Last Player Position` _stimuluslocation)
          (`KismetSystemLibrary.Delay` 1.0)
          (set `self.Enemy Audio Notified` false))))))

(event `self.ReceiveTick`
  (params (DeltaSeconds :type "Float (single-precision)"))
  (bind _player_in_range (`self.Player In Range`))
  (bind _returnvalue (`self.K2_GetActorLocation` (`self.Current Animal Actor`)))
  (`|ExecutionSequence`
    (:`then_0`
      (if (`self.Is Player Detected`)
        (set `self.Last Player Position` _returnvalue)
        (set `self.Is Player Near` (<= (`KismetMathLibrary.Vector_Distance` _returnvalue (`self.K2_GetActorLocation`)) (`self.Player Near Range`)))))
    (:`then_1`
      (if (`self.Is Enemy Detecting`)
        (bind _multiplier (`self.Get Detection Multiplier`))
        (bind _output_get (set `self.Current Detection Time` (+ (* _multiplier (`GameplayStatics.GetWorldDeltaSeconds`)) (`self.Current Detection Time`))))
        (if (>= _output_get (`self.Detection Time`))
          (set `self.Is Player Detected` true))
        (else
          (set `self.Current Detection Time` 0.0))))
    (:`then_2`
      (bind _asumg_detection_meter (cast `/Game/Blueprints/Widget/Enemies/UMG_DetectionMeter` (`WidgetComponent.GetUserWidgetObject` (`self.Detection Meter`))))
      (if (`self.Is Enemy Detecting`)
        (`/Game/Blueprints/Widget/Enemies/UMG_DetectionMeter.Show Meter` _asumg_detection_meter)
        (else
          (`/Game/Blueprints/Widget/Enemies/UMG_DetectionMeter.Hide Meter` _asumg_detection_meter))))
    (:`then_3`
      (`/Engine/EditorBlueprintResources/StandardMacros.IsValid` _player_in_range
        (:`Is Valid`
          (if (<= (`/Game/Blueprints/AI/BP_PlayerInRange.Total Players Inside` _player_in_range) 0)
            (set `self.Is Player Detected` false :!label _label)
            (set `self.Is Enemy Detecting` false)))
        (:`Is Not Valid`
          (goto _label))))))

(event `self.Animal Catcher.OnComponentBeginOverlap`
  (params (OverlappedComponent :type "PrimitiveComponent Object Reference") (OtherActor :type "Actor Object Reference") (OtherComp :type "PrimitiveComponent Object Reference") (OtherBodyIndex :type Integer) (bFromSweep :type Boolean) (SweepResult :type "HitResult Structure (by ref)"))
  (bind _asabanimal_character (cast `ABAnimalCharacter` OtherActor))
  (`ABAnimalCharacter.GetCaught` _asabanimal_character self))

(fn `Get Detection Multiplier`
  (returns (Multiplier :type "Float (double-precision)"))
  (`/Engine/EditorBlueprintResources/StandardMacros.IsValid` (`self.Current Animal Actor`)
    (:`Is Valid`
      (return (`KismetMathLibrary.MapRangeClamped` (`KismetMathLibrary.Vector_Distance` (`self.K2_GetActorLocation`) (`self.K2_GetActorLocation`)) (`self.Min Detecting Range`) (`self.Max Detection Range`) (`self.Max Detecting Rate`) (`self.Min Detection Rate`))))))

(fn `Get Patrol Point`
  (params (Index :type Integer))
  (returns (Location :type "Vector Structure"))
  (return (`self.K2_GetActorLocation` (`|GetArrayItem` (`self.Patrol Points`) (`KismetMathLibrary.Clamp` Index 0 (- (`KismetArrayLibrary.Array_Length` (`self.Patrol Points`)) 1))))))

(fn `Melee Attack`
  (returns (`Animation Duration` :type "Float (double-precision)"))
  (`KismetSystemLibrary.PrintString` "Melee Attack Player")
  (return (`self.Melee Duration`)))

(fn `Range Attack`
  (returns (`Animation Duration` :type "Float (double-precision)"))
  (`KismetSystemLibrary.PrintString` "Range Attack Player")
  (return (`self.Range Duration`)))

(fn `UserConstructionScript`)