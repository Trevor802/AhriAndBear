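; Crier enemy AI actor that senses animal characters and supplies patrol and hiding locations.
; Perception updates set the current animal and detection flag, and Tick records that animal's location as the last player position while detected.
; GetPatrolPoint returns a clamped-index patrol location.
; GetHidingPointAtDistance picks the hiding point with the longest path from the last player position, using a stored maximum that is never reset here.
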(event `self.ReceiveBeginPlay`
  (add `AIPerceptionComponent.OnTargetPerceptionUpdated` (`self.PerceptionComponent`) (delegate `OnTargetPerceptionUpdated_Event`)))

(event `OnTargetPerceptionUpdated_Event`
  (params (Actor :type "Actor Object Reference") (Stimulus :type "AIStimulus Structure"))
  (bind _asabanimal_character (cast `ABAnimalCharacter` Actor))
  (set `self.Current Animal Actor` _asabanimal_character)
  (set `self.Is Player Detected` (`.bSuccessfullySensed` (break `AIStimulus` Stimulus))))

(event `self.ReceiveTick`
  (params (DeltaSeconds :type "Float (single-precision)"))
  (`|ExecutionSequence`
    (:`then_0`
      (if (`self.Is Player Detected`)
        (set `self.Last Player Position` (`self.K2_GetActorLocation` (`self.Current Animal Actor`)))))))

(fn `GetHidingPointAtDistance`
  (returns (`Hiding Point` :type "Vector Structure"))
  (locals (`Current Farthest` :type "Vector Structure") (`Current Max Distance` :type "Float (double-precision)"))
  (for _array_element (`self.Hiding Points`)
    (bind _returnvalue (`self.K2_GetActorLocation` _array_element))
    (bind _pathlength (`NavigationSystemV1.GetPathLength` (`self.Last Player Position`) _returnvalue null null))
    (if (> _pathlength (`local.Current Max Distance`))
      (set `local.Current Farthest` _returnvalue)
      (set `local.Current Max Distance` _pathlength)))
  (return (`local.Current Farthest`)))

(fn `GetPatrolPoint`
  (params (Index :type Integer))
  (returns (FVector :type "Vector Structure"))
  (return (`self.K2_GetActorLocation` (`|GetArrayItem` (`self.Patrol Points`) (`KismetMathLibrary.Clamp` Index 0 (- (`KismetArrayLibrary.Array_Length` (`self.Patrol Points`)) 1))))))

(fn `UserConstructionScript`)