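; Playable animal character with survival stats (health, hunger, thirst, warmth) and input-driven movement: jog, crouch, prone, jump and a catch flag.
; A looping timer applies clamped stat changes, broadcasts updates and checks for death; ApplySurvivalEffect adjusts the same stats.
; Stats and transform are saved on BeginPlay or save events, and Restart sends load messages to all I_Saveable actors.
; CanDrainHealth gates health drain, but its depleted-stat check is unconnected.
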(event `InputAxis|WalkForward`
  (params (AxisValue :type "Float (single-precision)"))
  (if (not (`self.DisableMovement`))
    (`self.AddMovementInput` (`KismetMathLibrary.GetForwardVector` (`KismetMathLibrary.MakeRotator` 0.0 0.0 (.yaw (`self.GetControlRotation`)))) AxisValue)))

(event `InputAxis|WalkRight`
  (params (AxisValue :type "Float (single-precision)"))
  (if (not (`self.DisableMovement`))
    (`self.AddMovementInput` (`KismetMathLibrary.GetRightVector` (`KismetMathLibrary.MakeRotator` 0.0 0.0 (.yaw (`self.GetControlRotation`)))) AxisValue)))

(event `InputAxis|Turn`
  (params (AxisValue :type "Float (single-precision)"))
  (`self.AddControllerYawInput` AxisValue))

(event `InputAxis|LookUp`
  (params (AxisValue :type "Float (single-precision)"))
  (`self.AddControllerPitchInput` AxisValue))

(event `InputAction|Jump`
  (params (Key :type "Key Structure"))
  (bind _charactermovement (`self.CharacterMovement`))
  (:`Pressed`
    (if (`self.DisableMovement`)
      _
      (elif (`self.CrouchPressed`)
        (if (> (`CharacterMovementComponent.MaxWalkSpeed` (`self.CharacterMovement`)) 160.0)
          (if (> (`KismetMathLibrary.VSize` (`MovementComponent.Velocity` (`self.CharacterMovement`))) 0.0) :!label _label
            (if (`self.JogPressed`)
              (`self.Jump`)
              (set `CharacterMovementComponent.JumpZVelocity` (+ (`self.JumpHeight`) 100.0) _charactermovement)
              (else
                (`self.Jump`)
                (set `CharacterMovementComponent.JumpZVelocity` (`self.JumpHeight`) _charactermovement)))
            (set `self.JumpPressed` true)
            (else
              (`self.Jump`)
              (set `CharacterMovementComponent.JumpZVelocity` (`self.JumpHeight`) _charactermovement)
              (set `self.JumpPressed` true))))
        (else
          (goto _label)))))
  (:`Released`
    (set `self.JumpPressed` false)))

(event `InputAction|Jog`
  (params (Key :type "Key Structure"))
  (bind _charactermovement (`self.CharacterMovement`))
  (:`Pressed`
    (set `self.JogPressed` true)
    (set `CharacterMovementComponent.MaxWalkSpeed` (`self.SprintSpeed`) _charactermovement))
  (:`Released`
    (set `self.JogPressed` false)
    (if (`self.JogPressed`)
      (set `CharacterMovementComponent.MaxWalkSpeed` (`self.WalkSpeed`) _charactermovement)
      (else
        (set `CharacterMovementComponent.MaxWalkSpeed` (`self.RunSpeed`) _charactermovement)))))

(event `InputAction|Crouch`
  (params (Key :type "Key Structure"))
  (bind _charactermovement (`self.CharacterMovement`))
  (:`Pressed`
    (if (not (`self.PronePressed`))
      (`/Engine/EditorBlueprintResources/StandardMacros.FlipFlop`
        (:`A`
          (set `self.CrouchPressed` true)
          (set `CharacterMovementComponent.MaxWalkSpeed` (`self.WalkSpeed`) _charactermovement))
        (:`B`
          (set `self.CrouchPressed` false)
          (if (`self.JogPressed`)
            (set `CharacterMovementComponent.MaxWalkSpeed` (`self.SprintSpeed`) _charactermovement)
            (else
              (set `CharacterMovementComponent.MaxWalkSpeed` (`self.RunSpeed`) _charactermovement))))))))

(event `InputAction|Prone`
  (params (Key :type "Key Structure"))
  (:`Pressed`
    (if (not (`self.CrouchPressed`))
      (`/Engine/EditorBlueprintResources/StandardMacros.FlipFlop`
        (:`A`
          (set `self.PronePressed` true)
          (set `self.DisableMovement` true))
        (:`B`
          (set `self.PronePressed` false)
          (`KismetSystemLibrary.Delay` 1.4)
          (set `self.DisableMovement` false))))))

(event `InputAction|Catch`
  (params (Key :type "Key Structure"))
  (:`Pressed`
    (set `self.CatchPressed` true))
  (:`Released`
    (set `self.CatchPressed` false)))

(event `InputAction|Restart`
  (params (Key :type "Key Structure"))
  (:`Pressed`
    (bind _outactors (`GameplayStatics.GetAllActorsWithInterface` "/Game/Blueprints/GameMode/I_Saveable.I_Saveable_C"))
    (for _array_element _outactors
      (message `/Game/Blueprints/GameMode/I_Saveable.OnLoading` _array_element))
    (message `/Game/Blueprints/GameMode/I_Saveable.OnLoaded` _array_element true)
    (`self.OnRestarted`)))

(event `self.ReceiveBeginPlay`
  (`KismetSystemLibrary.K2_SetTimer` null "UpdateData" (`self.DataUpdateInverval`) true)
  (`self.SaveData`))

(event `/Game/Blueprints/GameMode/I_Saveable.OnSaving`
  (`self.SaveData`))

(event `/Game/Blueprints/GameMode/I_Saveable.OnLoading`
  (`self.LoadData`))

(fn `AddData`
  (params (Target :type "Float (double-precision) (by ref)") (Amount :type "Float (double-precision)" :default 1.0) (MaxValue :type "Float (double-precision)" :default 100.0))
  (locals (ResultValue :type "Float (double-precision)"))
  (bind _returnvalue (+ Target Amount))
  (if (> _returnvalue MaxValue)
    (set `local.ResultValue` MaxValue)
    (elif (< _returnvalue (`self.MinValue`))
      (set `local.ResultValue` (`self.MinValue`))
      (else
        (set `local.ResultValue` _returnvalue))))
  (`|VariableSetRef` Target (`local.ResultValue`)))

(fn `ApplySurvivalEffect`
  (params (Effect :type "/Game/Blueprints/Data/SurvivalData Structure"))
  (bind (_healtheffect _hungereffect _thirsteffect _warmtheffect) (break `/Game/Blueprints/Data/SurvivalData` Effect))
  (`self.AddData` (`self.Hunger`) _hungereffect (`self.MaxHunger`))
  (`self.AddData` (`self.Thirst`) _thirsteffect (`self.MaxThirst`))
  (`self.AddData` (`self.Warmth`) _warmtheffect (`self.Warmth`))
  (`self.AddData` (`self.Health`) _healtheffect (`self.MaxHealth`))
  (`self.CheckDeath`))

(fn `CheckDeath`
  (if (<= (`self.Health`) (`self.MinValue`))
    (`self.OnDead`)))

(fn `IsThirsty`
  (returns (bResult :type Boolean))
  (return (<= (`self.Thirst`) (`self.MinValue`))))

(fn `LoadData`
  (`|ExecutionSequence`
    (:`then_0`
      (set `self.Health` (`self.SavedHealth`))
      (set `self.Thirst` (`self.SavedThirst`))
      (set `self.Hunger` (`self.SavedHunger`))
      (set `self.Warmth` (`self.SavedWarmth`)))
    (:`then_1`
      (`self.K2_SetActorTransform` (`self.SavedTransform`)))))

(fn `ResetData`
  (set `self.Health` (`self.SavedHealth`))
  (set `self.Thirst` (`self.SavedThirst`))
  (set `self.Hunger` (`self.SavedHunger`))
  (set `self.Warmth` (`self.SavedWarmth`)))

(fn `SaveData`
  (`|ExecutionSequence`
    (:`then_0`
      (set `self.SavedHealth` (`self.Health`))
      (set `self.SavedThirst` (`self.Thirst`))
      (set `self.SavedHunger` (`self.Hunger`))
      (set `self.SavedWarmth` (`self.Warmth`)))
    (:`then_1`
      (set `self.SavedTransform` (`self.GetTransform`)))))

(fn `UpdateData`
  (`|ExecutionSequence`
    (:`then_0`
      (`self.AddData` (`self.Thirst`) (`self.ThirstDrainSpeed`))
      (`self.AddData` (`self.Hunger`) (`self.HungerDrainSpeed`))
      (`self.AddData` (`self.Warmth`) (`self.WarmthDrainSpeed`))
      (if (`self.CanDrainHealth`)
        (`self.AddData` (`self.Health`) (`self.HealthDrainSpeed`))))
    (:`then_1`
      (`self.OnDataUpdated`))
    (:`then_2`
      (`self.CheckDeath`))))

(fn `UserConstructionScript`)