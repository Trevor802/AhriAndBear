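; Playable cat character with a night-vision ability, hunger-driven camera focus and an AI follow behavior.
; Holding NightView sets the movement-disable flag and lowers first-person auto-exposure brightness limits to brighten dark scenes, restoring both on release.
; BeginPlay runs a camera fade, and UpdateData remaps third-person focus distance by hunger ratio.
; When the player controls the dog with following enabled, PawnSensing sends the cat toward the seen dog.
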(event `InputAction|NightView`
  (params (Key :type "Key Structure"))
  (:`Pressed`
    (set `self.DisableMovement` true)
    (set `self.NightViewOn` true)
    (set `CameraComponent.PostProcessSettings` (make `PostProcessSettings` :`AutoExposureMinBrightness` 0.3 :`AutoExposureMaxBrightness` 0.3) (`self.FPCam`)))
  (:`Released`
    (set `self.DisableMovement` false)
    (set `self.NightViewOn` false)
    (set `CameraComponent.PostProcessSettings` (make `PostProcessSettings` :`AutoExposureMinBrightness` 1.0 :`AutoExposureMaxBrightness` 1.0) (`self.FPCam`))))

(event `self.ReceiveBeginPlay`
  (`parent.ReceiveBeginPlay`)
  (`PlayerCameraManager.StartCameraFade` :`self` (`GameplayStatics.GetPlayerCameraManager` 0) :`FromAlpha` 1.0 :`Duration` 4.0 :`bHoldWhenFinished` true))

(event `self.ReceiveTick`
  (params (DeltaSeconds :type "Float (single-precision)"))
  (`parent.ReceiveTick` DeltaSeconds))

(event `self.UpdateData`
  (`parent.UpdateData`)
  (`self.UpdatePostProcess`))

(event `self.PawnSensing.OnSeePawn`
  (params (Pawn :type "Pawn Object Reference"))
  (bind _asbp_player_controller (cast `/Game/Blueprints/GameMode/BP_PlayerController` (`GameplayStatics.GetPlayerController` 0)))
  (if (and (`/Game/Blueprints/GameMode/BP_PlayerController.IsDog` _asbp_player_controller) (`/Game/Blueprints/GameMode/BP_PlayerController.IsFollowing` _asbp_player_controller))
    (bind _asbp_dog_character (cast `/Game/Blueprints/GameMode/BP_DogCharacter` Pawn))
    (`|AIMoveTo` self (-150.0 0.0 0.0) _asbp_dog_character)))

(fn `UpdatePostProcess`
  (set `CineCameraComponent.FocusSettings` (make `CameraFocusSettings` "Manual" (`KismetMathLibrary.Lerp` 200.0 900.0 (/ (`self.Hunger`) (`self.MaxHunger`))) (struct :`RelativeOffset` (0.0 0.0 0.0)) true) (`self.TPCam`)))

(fn `UserConstructionScript`
  (`parent.UserConstructionScript`))