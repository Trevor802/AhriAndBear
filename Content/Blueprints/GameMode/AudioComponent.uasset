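; Audio component for animal characters that plays sounds for barking, jumping, eating, abilities, character switching and survival stats.
; It binds to the owning animal's and player controller's events, playing action sounds at the animal's location.
; Ability, switch, hunger and moan sounds play in 2D only for the player's current character.
; Survival updates trigger hunger or moan cues as rounded percentages change, caching last values to limit repeats.
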(event `self.ReceiveBeginPlay`
  (bind _asbp_animal_character (cast `/Game/Blueprints/GameMode/BP_AnimalCharacter` (`self.GetOwner`)))
  (add `/Game/Blueprints/GameMode/BP_AnimalCharacter.OnBark` _asbp_animal_character (delegate `OnBark`))
  (add `/Game/Blueprints/GameMode/BP_AnimalCharacter.OnDataUpdated` _asbp_animal_character (delegate `OnDataUpdated`))
  (add `/Game/Blueprints/GameMode/BP_AnimalCharacter.OnJump` _asbp_animal_character (delegate `OnJump`))
  (add `/Game/Blueprints/GameMode/BP_AnimalCharacter.OnEat` _asbp_animal_character (delegate `OnEat`))
  (add `/Game/Blueprints/GameMode/BP_AnimalCharacter.OnActivateAbility` _asbp_animal_character (delegate `OnActivateAbility`))
  (bind _asbp_player_controller (cast `/Game/Blueprints/GameMode/BP_PlayerController` (`GameplayStatics.GetPlayerController` 0)))
  (add `/Game/Blueprints/GameMode/BP_PlayerController.OnCharacterSwitched` _asbp_player_controller (delegate `OnSwitchCharacter`)))

(event `OnActivateAbility`
  (`self.Play2D` (`self.ActivateAbilitySound`)))

(event `OnEat`
  (`self.PlayAtPlayer` (`self.EatSound`)))

(event `OnBark`
  (params (Position :type "Vector Structure"))
  (`self.PlayAtPlayer` (`self.CallSound`)))

(event `OnDataUpdated`
  (params (NewData :type "/Game/Blueprints/Data/SurvivalData Structure"))
  (`self.UpdateSurvivalDataSound` NewData))

(event `OnJump`
  (`self.PlayAtPlayer` (`self.JumpSound`)))

(event `OnSwitchCharacter`
  (params (NewAnimal :type "/Game/Blueprints/Data/E_AnimalType Enum" :default "NewEnumerator0"))
  (`self.Play2D` (`self.SwitchCharacterSound`)))

(fn `Play2D`
  (params (Sound :type "SoundBase Object Reference"))
  (if (== (`self.GetOwner`) (`GameplayStatics.GetPlayerCharacter` 0))
    (`GameplayStatics.PlaySound2D` Sound 1.0 1.0 0.0 null null)))

(fn `PlayAtPlayer`
  (params (Sound :type "SoundBase Object Reference"))
  (`GameplayStatics.PlaySoundAtLocation` Sound (`self.GetAnimalLocation`) (struct) 1.0 1.0 0.0 null null null))

(fn `TryPlayHungry`
  (params (HungerPct :type Integer))
  (bind _returnvalue (`self.RoundToTen` HungerPct))
  (if (or (and (<= _returnvalue 50) (!= _returnvalue (`self.LastPlayHungerValue`))) (<= HungerPct 0))
    (`self.Play2D` (`self.HungrySound`))
    (set `self.LastPlayHungerValue` _returnvalue)))

(fn `TryPlayMoanEveryTen`
  (params (MoanValuePct :type Integer) (LastPlayValue :type "Integer (by ref)"))
  (bind _returnvalue (`self.RoundToTen` MoanValuePct))
  (if (or (!= _returnvalue LastPlayValue) (<= MoanValuePct 0))
    (`self.Play2D` (`self.MoanSound`))
    (`|VariableSetRef` LastPlayValue _returnvalue)))

(fn `UpdateSurvivalDataSound`
  (params (SurvivalData :type "/Game/Blueprints/Data/SurvivalData Structure (by ref)"))
  (bind (_health _hunger _thirst _warmth) (break `/Game/Blueprints/Data/SurvivalData` SurvivalData))
  (bind _asbp_animal_character (`self.GetAnimalOwner`))
  (`self.TryPlayHungry` (`self.GetPercentage` _hunger (`/Game/Blueprints/GameMode/BP_AnimalCharacter.MaxHunger` _asbp_animal_character)))
  (`self.TryPlayMoanEveryTen` (`self.GetPercentage` _thirst (`/Game/Blueprints/GameMode/BP_AnimalCharacter.MaxThirst` _asbp_animal_character)) (`self.LastMoanByThirst`))
  (`self.TryPlayMoanEveryTen` (`self.GetPercentage` _warmth (`/Game/Blueprints/GameMode/BP_AnimalCharacter.Warmth` _asbp_animal_character)) (`self.LastMoanByWarmth`)))