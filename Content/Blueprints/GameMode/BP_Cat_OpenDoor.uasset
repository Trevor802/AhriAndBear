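; Playable cat character that can unlock a BP_Door it overlaps when Catch is pressed.
; The ability toggle changes first-person camera exposure brightness limits, and BeginPlay starts a camera fade from black.
; UpdateData emits noise, while pawn sensing moves the cat to the dog when the player controller's IsDog and IsFollowing are set.
; An interactive-object outline trace using material parameters is present but never runs.
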(event `self.OnSwitchAbility`
  (params (AbilityOn :type Boolean))
  (bind _fpcam (`self.FPCam`))
  (if AbilityOn
    (set `CameraComponent.PostProcessSettings` (make `PostProcessSettings` :`AutoExposureMinBrightness` 0.1 :`AutoExposureMaxBrightness` 0.1) _fpcam)
    (else
      (set `CameraComponent.PostProcessSettings` (make `PostProcessSettings`) _fpcam))))

(event `self.ReceiveBeginPlay`
  (`parent.ReceiveBeginPlay`)
  (`PlayerCameraManager.StartCameraFade` :`self` (`GameplayStatics.GetPlayerCameraManager` 0) :`FromAlpha` 1.0 :`Duration` 4.0 :`bHoldWhenFinished` true))

(event `self.ReceiveActorBeginOverlap`
  (params (OtherActor :type "Actor Object Reference"))
  ;[1 0.8634 0.1718] Is it in use?
  (`parent.ReceiveActorBeginOverlap` OtherActor)
  (cast `/Game/Blueprints/InteractiveObjects/BP_Door` OtherActor)
  (set `self.CanInteract` true))

(event `InputAction|Catch`
  (params (Key :type "Key Structure"))
  (:`Pressed`
    (if (`self.CanInteract`)
      (bind _asbp_door (cast `/Game/Blueprints/InteractiveObjects/BP_Door` (stale `self.ReceiveActorBeginOverlap` OtherActor)))
      (`/Game/Blueprints/InteractiveObjects/BP_Door.Unlock` _asbp_door))))

(event `self.ReceiveActorEndOverlap`
  (params (OtherActor :type "Actor Object Reference"))
  (cast `/Game/Blueprints/InteractiveObjects/BP_Door` OtherActor)
  (set `self.CanInteract` false))

(event `self.ReceiveTick`
  (params (DeltaSeconds :type "Float (single-precision)"))
  (`parent.ReceiveTick` DeltaSeconds))

(event `self.UpdateData`
  (`parent.UpdateData`)
  (`PawnNoiseEmitterComponent.MakeNoise` (`self.PawnNoiseEmitter`) self 1.0 (`self.K2_GetActorLocation`)))

(event `self.PawnSensing.OnSeePawn`
  (params (Pawn :type "Pawn Object Reference"))
  (bind _asbp_player_controller (cast `/Game/Blueprints/GameMode/BP_PlayerController` (`GameplayStatics.GetPlayerController` 0)))
  (if (and (`/Game/Blueprints/GameMode/BP_PlayerController.IsDog` _asbp_player_controller) (`/Game/Blueprints/GameMode/BP_PlayerController.IsFollowing` _asbp_player_controller))
    (bind _asbp_dog_character (cast `/Game/Blueprints/GameMode/BP_DogCharacter` Pawn))
    (`|AIMoveTo` self (0.0 0.0 0.0) _asbp_dog_character 1.0
      (:`OnFail`
        (`KismetSystemLibrary.PrintString` "Hello")))))

(event `self.PawnSensing.OnHearNoise`
  (params (Instigator :type "Pawn Object Reference") (Location :type "Vector Structure (by ref)") (Volume :type "Float (single-precision)"))
  (bind _asbp_player_controller (cast `/Game/Blueprints/GameMode/BP_PlayerController` (`GameplayStatics.GetPlayerController` 0)))
  (if (and (`/Game/Blueprints/GameMode/BP_PlayerController.IsDog` _asbp_player_controller) (`/Game/Blueprints/GameMode/BP_PlayerController.IsFollowing` _asbp_player_controller))
    (bind _asbp_dog_character (cast `/Game/Blueprints/GameMode/BP_DogCharacter` Instigator))
    (`|AIMoveTo` self (0.0 0.0 0.0) _asbp_dog_character 1.0)))

(fn `UserConstructionScript`
  (`parent.UserConstructionScript`))