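; Player controller for a game where the player swaps between a dog and a cat character.
; On begin play it finds both animals, broadcasts which one is controlled, and briefly blends the camera to a checkpoint before blending back to the player.
; The ChangeAnimal input swaps possession between player and AI controllers and broadcasts the switch.
; The AnimalTogether input toggles a following flag.
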(event `self.ReceiveBeginPlay`
  (bind (_asbp_dog_character _bsuccess) (cast `/Game/Blueprints/GameMode/BP_DogCharacter` (`GameplayStatics.GetPlayerCharacter` 0) :!pure true))
  (bind _returnvalue (`GameplayStatics.GetActorOfClass` "/Game/Blueprints/GameMode/BP_DogCharacter.BP_DogCharacter_C"))
  (set `self.Dog` _returnvalue)
  (bind _returnvalue_2 (`GameplayStatics.GetActorOfClass` "/Game/Blueprints/GameMode/BP_CatCharacter.BP_CatCharacter_C"))
  (set `self.Cat` _returnvalue_2)
  (`self.OnCharacterSwitched` _bsuccess)
  (set `self.IsDog` _bsuccess)
  (bind _returnvalue_3 (`GameplayStatics.GetActorOfClass` "/Game/Blueprints/InteractiveObjects/BP_Checkpoint.BP_Checkpoint_C"))
  (`self.SetViewTargetWithBlend` _returnvalue_3 1.0)
  (`KismetSystemLibrary.Delay` 2.0)
  (`self.SetViewTargetWithBlend` (`GameplayStatics.GetPlayerController` 0) 3.0))

(event `InputAction|ChangeAnimal`
  (params (Key :type "Key Structure"))
  (:`Pressed`
    (if (`self.IsDog`)
      (`self.Possess` (`AIBlueprintHelperLibrary.GetAIController` (`self.Cat`)) (`self.Dog`))
      (`self.Possess` (`GameplayStatics.GetPlayerController` 0) (`self.Cat`))
      (else
        (`self.Possess` (`AIBlueprintHelperLibrary.GetAIController` (`self.Dog`)) (`self.Cat`))
        (`self.Possess` (`GameplayStatics.GetPlayerController` 0) (`self.Dog`))))
    (bind _output_get (set `self.IsDog` (not (`self.IsDog`))))
    (`self.OnCharacterSwitched` _output_get)))

(event `InputAction|AnimalTogether`
  (params (Key :type "Key Structure"))
  (:`Pressed`
    (set `self.IsFollowing` (not (`self.IsFollowing`)))))

(fn `UserConstructionScript`)