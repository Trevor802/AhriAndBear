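; Player controller that lets the player switch control between a dog and a cat character.
; BeginPlay caches both characters and fires the OnCharacterSwitched dispatcher with false.
; ChangeAnimal swaps possession between player controller 0 and the other animal's AI controller, flips IsDog and broadcasts the new state.
; AnimalTogether toggles an IsFollowing flag, which nothing in this graph reads.
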(event `self.ReceiveBeginPlay`
  (bind _returnvalue (`GameplayStatics.GetActorOfClass` "/Game/Blueprints/GameMode/BP_DogCharacter.BP_DogCharacter_C"))
  (set `self.Dog` _returnvalue)
  (bind _returnvalue_2 (`GameplayStatics.GetActorOfClass` "/Game/Blueprints/GameMode/BP_CatCharacter.BP_CatCharacter_C"))
  (set `self.Cat` _returnvalue_2)
  (`self.OnCharacterSwitched` false))

(event `InputAction|AnimalTogether`
  (params (Key :type "Key Structure"))
  (:`Pressed`
    (set `self.IsFollowing` (not (`self.IsFollowing`)))))

(event `InputAction|ChangeAnimal`
  (params (Key :type "Key Structure"))
  (:`Pressed`
    (if (`self.IsDog`)
      (`self.Possess` (`AIBlueprintHelperLibrary.GetAIController` (`self.Cat`)) (`self.Dog`))
      (`self.Possess` (`GameplayStatics.GetPlayerController` 0) (`self.Cat`))
      (else
        (`self.Possess` (`AIBlueprintHelperLibrary.GetAIController` (`self.Dog`)) (`self.Cat`))
        (`self.Possess` (`GameplayStatics.GetPlayerController` 0) (`self.Dog`))))
    (bind _output_get (set `self.IsDog` (not (`self.IsDog`))))
    (`self.OnCharacterSwitched` _output_get)))

(fn `UserConstructionScript`)