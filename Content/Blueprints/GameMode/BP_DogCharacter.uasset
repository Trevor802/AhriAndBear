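; BP_DogCharacter is the dog character, which can follow the cat character under AI movement.
; When its PawnSensing component sees a pawn, it checks that the player controller's IsDog is false and IsFollowing is true.
; If the seen pawn is a BP_CatCharacter, it issues an AIMoveTo with that cat as the target actor.
; Movement is triggered only by sight events, with no Tick logic.
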(event `self.ReceiveBeginPlay`
  (`parent.ReceiveBeginPlay`))

(event `self.PawnSensing.OnSeePawn`
  (params (Pawn :type "Pawn Object Reference"))
  (bind _asbp_player_controller (cast `/Game/Blueprints/GameMode/BP_PlayerController` (`GameplayStatics.GetPlayerController` 0)))
  (if (and (not (`/Game/Blueprints/GameMode/BP_PlayerController.IsDog` _asbp_player_controller)) (`/Game/Blueprints/GameMode/BP_PlayerController.IsFollowing` _asbp_player_controller))
    (bind _asbp_cat_character (cast `/Game/Blueprints/GameMode/BP_CatCharacter` Pawn))
    (`|AIMoveTo` self (-150.0 0.0 0.0) _asbp_cat_character)))

(fn `UserConstructionScript`
  (`parent.UserConstructionScript`))