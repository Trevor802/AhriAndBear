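; Trigger actor that streams levels in and out when an ABAnimalCharacter overlaps its collision component.
; On overlap it starts loading LevelsToLoad as visible, blocking loads, then after a short delay starts unloading LevelsToUnload without blocking.
; Both events walk their soft-reference arrays one latent call at a time through a shared Index, then reset it and disable collision to stop further triggering.
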(event `self.CollisionComponent.OnComponentBeginOverlap`
  (params (OverlappedComponent :type "PrimitiveComponent Object Reference") (OtherActor :type "Actor Object Reference") (OtherComp :type "PrimitiveComponent Object Reference") (OtherBodyIndex :type Integer) (bFromSweep :type Boolean) (SweepResult :type "HitResult Structure (by ref)"))
  (cast `ABAnimalCharacter` OtherActor)
  (`self.DoLoading`)
  (`KismetSystemLibrary.Delay` 2.0)
  (`self.DoUnloading`))

(event `DoLoading`
  (bind _levelstoload (`self.LevelsToLoad`))
  (if (< (`self.Index`) (`KismetArrayLibrary.Array_Length` _levelstoload)) :!label _label
    (`GameplayStatics.LoadStreamLevelBySoftObjectPtr` (`|GetArrayItem` _levelstoload (`self.Index`)) true true)
    (`/Engine/EditorBlueprintResources/StandardMacros.IncrementInt` (`self.Index`)
      (:`  `
        (goto _label)))
    (else
      (set `self.Index` 0)
      ;[1 1 1] Disable collision triggered loading n unloading
      (`PrimitiveComponent.SetCollisionEnabled` (`self.CollisionComponent`) "NoCollision" :!label _label_2))))

(event `DoUnloading`
  (bind _levelstounload (`self.LevelsToUnload`))
  (if (< (`self.Index`) (`KismetArrayLibrary.Array_Length` _levelstounload)) :!label _label_3
    (`GameplayStatics.UnloadStreamLevelBySoftObjectPtr` (`|GetArrayItem` _levelstounload (`self.Index`)))
    (`/Engine/EditorBlueprintResources/StandardMacros.IncrementInt` (`self.Index`)
      (:`  `
        (goto _label_3)))
    (else
      (set `self.Index` 0)
      (goto _label_2))))

(fn `UserConstructionScript`)