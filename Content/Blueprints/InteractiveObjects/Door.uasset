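; Interactive door that takes the cat and dog characters to open, each acting only while falling on overlap.
; While locked, an airborne cat overlapping the door unlocks it.
; Once unlocked, an airborne dog overlapping it nudges the rotation toward a fixed target.
; The RInterpTo runs once per overlap with a constant delta time, so each hit moves the door one small step instead of animating it.
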(event `self.ReceiveTick`
  (params (DeltaSeconds :type "Float (single-precision)")))

(event `self.ReceiveActorBeginOverlap`
  (params (OtherActor :type "Actor Object Reference"))
  (if (`self.IsLocked`)
    (bind _asbp_cat_character (cast `/Game/Blueprints/GameMode/BP_CatCharacter` OtherActor))
    (if (`NavMovementComponent.IsFalling` (`Character.CharacterMovement` _asbp_cat_character))
      (set `self.IsLocked` false))
    (else
      (bind _asbp_dog_character (cast `/Game/Blueprints/GameMode/BP_DogCharacter` OtherActor))
      (if (`NavMovementComponent.IsFalling` (`Character.CharacterMovement` _asbp_dog_character))
        (`self.K2_SetActorRotation` (`KismetMathLibrary.RInterpTo` (`self.K2_GetActorRotation`) (struct :`Yaw` 40.0) 0.2 0.3))))))

(fn `UserConstructionScript`)