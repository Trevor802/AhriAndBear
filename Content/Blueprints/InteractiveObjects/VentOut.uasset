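; VentOut is an interactive-object Blueprint with a floating info marker; the graph only drives that widget, with no vent interaction logic.
; BeginPlay sets the label text.
; Every Tick updates the player distance in meters, replays one of two widget animations by a distance threshold, and hides the marker at very close range.
; A Timeline, played from Tick, shifts the widget vertically, turns it toward the player and applies a boosted color tint.
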(event `self.ReceiveBeginPlay`
  ;[1 1 1] UI Words change
  (bind _asfloating_information_umg (cast `/Game/Assets/UMG/Widget/FloatingInformationUMG` (`WidgetComponent.GetUserWidgetObject` (`self.Widget`))))
  (`TextBlock.SetText` (`/Game/Assets/UMG/Widget/FloatingInformationUMG.TextBlock_51` _asfloating_information_umg) (`KismetTextLibrary.Conv_StringToText` (`self.UI Sentence`))))

(event `self.ReceiveTick`
  (params (DeltaSeconds :type "Float (single-precision)"))
  (bind _widget (`self.Widget`))
  (bind _returnvalue (`SceneComponent.K2_GetComponentLocation` (`self.Widget`)))
  (bind _returnvalue_2 (`WidgetComponent.GetUserWidgetObject` (`self.Widget`)))
  (bind _returnvalue_3 (`KismetMathLibrary.Vector_Distance` (`self.K2_GetActorLocation` (`GameplayStatics.GetPlayerPawn` 0)) (`SceneComponent.K2_GetComponentLocation` (`self.Widget`))))
  (`|ExecutionSequence`
    (:`then_1`
      ;[1 1 1] Display Distance Change
      (set `self.distance` _returnvalue_3)
      (bind _asfloating_information_umg (cast `/Game/Assets/UMG/Widget/FloatingInformationUMG` (`WidgetComponent.GetUserWidgetObject` (`self.Widget`))))
      (`TextBlock.SetText` (`/Game/Assets/UMG/Widget/FloatingInformationUMG.Distance` _asfloating_information_umg) (`KismetTextLibrary.Conv_StringToText` (`KismetStringLibrary.Concat_StrStr` (`KismetTextLibrary.Conv_TextToString` (`KismetTextLibrary.Conv_DoubleToText` (/ _returnvalue_3 100.0) "HalfToEven" false true 1 324 0 1)) "M"))))
    (:`then_2`
      ;[1 1 1] Toward Player
      (bind (_direction `_新建轨迹_0`) (`Timeline|时间轴_0`)
        (:`Update`
          (`SceneComponent.K2_SetWorldLocation` (`self.Widget`) (`KismetMathLibrary.MakeVector` (.x _returnvalue) (.y _returnvalue) (+ (.z _returnvalue) (* `_新建轨迹_0` 0.5))) false false)
          (`SceneComponent.K2_SetWorldRotation` (`self.Widget`) (`KismetMathLibrary.FindLookAtRotation` _returnvalue (`self.K2_GetActorLocation` (`GameplayStatics.GetPlayerPawn` 0))) false false)
          (`WidgetComponent.SetTintColorAndOpacity` (`self.Widget`) (* (`self.UI Color`) 10.0)))))
    (:`then_3`
      ;[1 1 1] WidgetAnimationChange
      (if (<= (`self.Distance`) (`self.Widget Animation Change Distance Control`))
        (bind _asfloating_information_umg_2 (cast `/Game/Assets/UMG/Widget/FloatingInformationUMG` _returnvalue_2))
        (`UserWidget.PlayAnimation` _asfloating_information_umg_2 (`/Game/Assets/UMG/Widget/FloatingInformationUMG.Acticed` _asfloating_information_umg_2) 0.0 1 "Forward" 1.0)
        (else
          (bind _asfloating_information_umg_3 (cast `/Game/Assets/UMG/Widget/FloatingInformationUMG` _returnvalue_2))
          (`UserWidget.PlayAnimation` _asfloating_information_umg_3 (`/Game/Assets/UMG/Widget/FloatingInformationUMG.InDistance` _asfloating_information_umg_3) 0.0 1 "Forward" 1.0))))
    (:`then_4`
      ;[1 1 1] Too close, Disappear
      (if (<= (`self.Distance`) 50.0)
        (`SceneComponent.SetVisibility` _widget false false)
        (else
          (`SceneComponent.SetVisibility` _widget true false))))))

(fn `UserConstructionScript`)