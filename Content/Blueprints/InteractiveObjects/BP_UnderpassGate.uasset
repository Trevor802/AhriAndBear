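; BP_UnderpassGate is an interactive underpass gate that moves its static mesh between begin and end switch positions.
; When opening begins, the SwitchOn timeline plays from the start, and its offset curve linearly interpolates the mesh's relative location.
; When the door-opened event fires, it stops the timeline and snaps the mesh to the end or begin position according to the result.
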(event `self.OnBeginOpen`
  (bind (_direction _switchoffsetcurve) (`Timeline|SwitchOn` :!via `PlayFromStart` :!label _label)
    (:`Update`
      (`SceneComponent.K2_SetRelativeLocation` (`self.StaticMesh`) (`|EaseFunction` "Linear" _switchoffsetcurve (`self.SwitchBeginPos`) (`self.SwitchEndPos`)) false false))))

(event `self.OnDoorOpened`
  (params (bResult :type Boolean))
  (`|ExecutionSequence`
    (:`then_0`
      (goto _label :!via `Stop`))
    (:`then_1`
      (`SceneComponent.K2_SetRelativeLocation` (`self.StaticMesh`) (`KismetMathLibrary.SelectVector` (`self.SwitchEndPos`) (`self.SwitchBeginPos`) bResult) false false))))

(fn `UserConstructionScript`
  (`parent.UserConstructionScript`))