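; BP_Pizza is an interactive pizza object that highlights its food meshes while a dog or cat character is nearby.
; Begin overlap on InteractCollision by either character enables custom depth and sets a stencil value on the three food meshes.
; End overlap by either character turns it off, without checking whether the other is still inside.
; The file holds only this highlight logic, with an empty construction script.
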(event `self.InteractCollision.OnComponentBeginOverlap`
  (params (OverlappedComponent :type "PrimitiveComponent Object Reference") (OtherActor :type "Actor Object Reference") (OtherComp :type "PrimitiveComponent Object Reference") (OtherBodyIndex :type Integer) (bFromSweep :type Boolean) (SweepResult :type "HitResult Structure (by ref)"))
  (bind _foodmesh1 (`self.FoodMesh1`))
  (cast `/Game/Blueprints/Characters/BP_NewDogCharacter` OtherActor
    (:`then`
      _)
    (:`CastFailed`
      (cast `/Game/Blueprints/Characters/BP_NewCatCharacter` OtherActor)))
  (`PrimitiveComponent.SetRenderCustomDepth` _foodmesh1 true)
  (`PrimitiveComponent.SetRenderCustomDepth` (`self.FoodMesh2`) true)
  (`PrimitiveComponent.SetRenderCustomDepth` (`self.FoodMesh3`) true)
  (`PrimitiveComponent.SetCustomDepthStencilValue` _foodmesh1 2)
  (`PrimitiveComponent.SetCustomDepthStencilValue` (`self.FoodMesh2`) 2)
  (`PrimitiveComponent.SetCustomDepthStencilValue` (`self.FoodMesh3`) 2))

(event `self.InteractCollision.OnComponentEndOverlap`
  (params (OverlappedComponent :type "PrimitiveComponent Object Reference") (OtherActor :type "Actor Object Reference") (OtherComp :type "PrimitiveComponent Object Reference") (OtherBodyIndex :type Integer))
  (bind _foodmesh1 (`self.FoodMesh1`))
  (cast `/Game/Blueprints/Characters/BP_NewDogCharacter` OtherActor
    (:`then`
      _)
    (:`CastFailed`
      (cast `/Game/Blueprints/Characters/BP_NewCatCharacter` OtherActor)))
  (`PrimitiveComponent.SetRenderCustomDepth` _foodmesh1 false)
  (`PrimitiveComponent.SetRenderCustomDepth` (`self.FoodMesh2`) false)
  (`PrimitiveComponent.SetRenderCustomDepth` (`self.FoodMesh3`) false)
  (`PrimitiveComponent.SetCustomDepthStencilValue` _foodmesh1 0)
  (`PrimitiveComponent.SetCustomDepthStencilValue` (`self.FoodMesh2`) 0)
  (`PrimitiveComponent.SetCustomDepthStencilValue` (`self.FoodMesh3`) 0))

(fn `UserConstructionScript`)