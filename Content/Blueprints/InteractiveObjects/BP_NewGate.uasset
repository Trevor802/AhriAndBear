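; BP_NewGate is an interactive gate object with a floating information widget that shows a label and a distance readout.
; BeginPlay sets the widget's text and tint from UIText and UIColor.
; Each Tick writes Distance in meters to the widget and replays its Acticed or InDistance animation depending on the WidigetChangeDistance threshold.
; Distance is only read here, and no gate opening logic is present.
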(event `self.ReceiveBeginPlay`
  (bind _uiwidget (`self.UIWidget`))
  ;[1 1 1] UI Words change
  (bind _asfloating_information_umg (cast `/Game/Assets/UMG/Widget/FloatingInformationUMG` (`WidgetComponent.GetUserWidgetObject` _uiwidget)))
  (`TextBlock.SetText` (`/Game/Assets/UMG/Widget/FloatingInformationUMG.TextBlock_51` _asfloating_information_umg) (`KismetTextLibrary.Conv_StringToText` (`self.UIText`)))
  (`WidgetComponent.SetTintColorAndOpacity` _uiwidget (`self.UIColor`)))

(event `self.ReceiveTick`
  (params (DeltaSeconds :type "Float (single-precision)"))
  (bind _returnvalue (`WidgetComponent.GetUserWidgetObject` (`self.UIWidget`)))
  (`|ExecutionSequence`
    (:`then_0`
      ;[1 1 1] Display Distance Change
      (bind _asfloating_information_umg (cast `/Game/Assets/UMG/Widget/FloatingInformationUMG` (`WidgetComponent.GetUserWidgetObject` (`self.UIWidget`))))
      (`TextBlock.SetText` (`/Game/Assets/UMG/Widget/FloatingInformationUMG.Distance` _asfloating_information_umg) (`KismetTextLibrary.Conv_StringToText` (`KismetStringLibrary.Concat_StrStr` (`KismetTextLibrary.Conv_TextToString` (`KismetTextLibrary.Conv_DoubleToText` (`self.Distance`) "HalfToEven" false true 1 324 0 1)) "M"))))
    (:`then_1`
      ;[1 1 1] WidgetAnimationChange
      (if (<= (`self.Distance`) (`self.WidigetChangeDistance`))
        (bind _asfloating_information_umg_2 (cast `/Game/Assets/UMG/Widget/FloatingInformationUMG` _returnvalue))
        (`UserWidget.PlayAnimation` _asfloating_information_umg_2 (`/Game/Assets/UMG/Widget/FloatingInformationUMG.Acticed` _asfloating_information_umg_2) 0.0 1 "Forward" 1.0 false)
        (else
          (bind _asfloating_information_umg_3 (cast `/Game/Assets/UMG/Widget/FloatingInformationUMG` _returnvalue))
          (`UserWidget.PlayAnimation` _asfloating_information_umg_3 (`/Game/Assets/UMG/Widget/FloatingInformationUMG.InDistance` _asfloating_information_umg_3) 0.0 1 "Forward" 1.0 false))))))

(fn `UserConstructionScript`)