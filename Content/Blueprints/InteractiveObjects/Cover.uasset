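; Interactive cover actor that toggles a Fresnel highlight when the player comes near.
; Each tick it compares the player pawn's distance to its Cylinder against the OutlineDistance value from a Material Parameter Collection plus a fixed margin.
; It writes the result to the collection's Cover_EnabledFresnel scalar, which is global, so all cover instances share and overwrite the same flag.
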(event `self.ReceiveTick`
  (params (DeltaSeconds :type "Float (single-precision)"))
  (bind _returnvalue (`KismetMaterialLibrary.GetScalarParameterValue` "/Game/Assets/MPC/MPC.MPC" "OutlineDistance"))
  (if (<= (`KismetMathLibrary.Vector_Distance` (`self.K2_GetActorLocation` (`GameplayStatics.GetPlayerPawn` 0)) (`SceneComponent.K2_GetComponentLocation` (`self.Cylinder`))) (+ _returnvalue 250.0))
    (`KismetMaterialLibrary.SetScalarParameterValue` "/Game/Assets/MPC/MPC.MPC" "Cover_EnabledFresnel" 1.0)
    (else
      (`KismetMaterialLibrary.SetScalarParameterValue` "/Game/Assets/MPC/MPC.MPC" "Cover_EnabledFresnel"))))

(event `self.ReceiveBeginPlay`)

(fn `UserConstructionScript`)