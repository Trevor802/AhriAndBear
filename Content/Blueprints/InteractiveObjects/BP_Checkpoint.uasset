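; Checkpoint actor that triggers a game-wide save when a BP_AnimalCharacter enters its box.
; Begin overlap sets CanSave and calls TrySave, which checks CanInteract and fires OnInteracting; end overlap clears the flag.
; OnInteracting sends OnSavingMessage to every actor implementing I_Saveable, leaving each to handle its own saving.
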(event `self.OnInteracting`
  (bind _outactors (`GameplayStatics.GetAllActorsWithInterface` "/Game/Blueprints/GameMode/I_Saveable.I_Saveable_C"))
  (for _array_element _outactors
    (message `/Game/Blueprints/GameMode/I_Saveable.OnSaving` _array_element)))

(event `self.Box.OnComponentBeginOverlap`
  (params (OverlappedComponent :type "PrimitiveComponent Object Reference") (OtherActor :type "Actor Object Reference") (OtherComp :type "PrimitiveComponent Object Reference") (OtherBodyIndex :type Integer) (bFromSweep :type Boolean) (SweepResult :type "HitResult Structure (by ref)"))
  (cast `/Game/Blueprints/GameMode/BP_AnimalCharacter` OtherActor)
  (set `self.bCanSave` true)
  (`self.TrySave`))

(event `self.Box.OnComponentEndOverlap`
  (params (OverlappedComponent :type "PrimitiveComponent Object Reference") (OtherActor :type "Actor Object Reference") (OtherComp :type "PrimitiveComponent Object Reference") (OtherBodyIndex :type Integer))
  (cast `/Game/Blueprints/GameMode/BP_AnimalCharacter` OtherActor)
  (set `self.bCanSave` false))

(fn `CanInteract`
  (returns (Result :type Boolean))
  (return (`self.bCanSave`)))

(fn `TrySave`
  (bind _result (`self.CanInteract`))
  (if _result
    (`self.OnInteracting`)))

(fn `UserConstructionScript`)