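; Interactive water bowl that an animal character can drink from to receive a survival effect.
; Each tick it toggles a Fresnel highlight through a Material Parameter Collection, based on player distance and the shared outline distance.
; When an overlapping animal presses catch, its movement locks for a short delay.
; It then consumes water and applies the effect through ItemComponent if enough remains, and movement unlocks either way.
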(event `self.ReceiveBeginPlay`
  (set `self.SurvivalEffect` (make `/Game/Blueprints/Data/SurvivalData` 0.0 0.0 (`self.WaterReduce`))))

(event `self.Box.OnComponentBeginOverlap`
  (params (OverlappedComponent :type "PrimitiveComponent Object Reference") (OtherActor :type "Actor Object Reference") (OtherComp :type "PrimitiveComponent Object Reference") (OtherBodyIndex :type Integer) (bFromSweep :type Boolean) (SweepResult :type "HitResult Structure (by ref)"))
  (bind _asbp_animal_character (cast `/Game/Blueprints/GameMode/BP_AnimalCharacter` OtherActor))
  (set `self.Animal` _asbp_animal_character)
  (set `self.IsOverlapping` true))

(event `self.Box.OnComponentEndOverlap`
  (params (OverlappedComponent :type "PrimitiveComponent Object Reference") (OtherActor :type "Actor Object Reference") (OtherComp :type "PrimitiveComponent Object Reference") (OtherBodyIndex :type Integer))
  (cast `/Game/Blueprints/GameMode/BP_AnimalCharacter` OtherActor)
  (set `self.IsOverlapping` false))

(event `self.ReceiveTick`
  (params (DeltaSeconds :type "Float (single-precision)"))
  (bind _returnvalue (`KismetMaterialLibrary.GetScalarParameterValue` "/Game/Assets/MPC/MPC.MPC" "OutlineDistance"))
  (if (<= (`KismetMathLibrary.Vector_Distance` (`SceneComponent.K2_GetComponentLocation` (`self.Box`)) (`self.K2_GetActorLocation` (`GameplayStatics.GetPlayerPawn` 0))) (+ _returnvalue 250.0))
    (`KismetMaterialLibrary.SetScalarParameterValue` "/Game/Assets/MPC/MPC.MPC" "Bowl_EnabledFresnel" 1.0)
    (else
      (`KismetMaterialLibrary.SetScalarParameterValue` "/Game/Assets/MPC/MPC.MPC" "Bowl_EnabledFresnel")))
  (bind _result (`self.CanInteract`))
  (if _result
    (`self.OnInteracting`)
    (`KismetSystemLibrary.Delay` 2.0)
    (`self.OnInteracted` false)))

(event `self.OnInteracting`
  (set `/Game/Blueprints/GameMode/BP_AnimalCharacter.DisableMovement` true (`self.Animal`)))

(event `self.OnInteracted`
  (params (bResult :type Boolean))
  (bind _returnvalue (- (`self.WaterAmount`) (`self.WaterReduce`)))
  (if (>= _returnvalue 0.0)
    (set `self.WaterAmount` _returnvalue)
    (`/Game/Blueprints/GameMode/ItemComponent.EatItem` (`self.ItemComponent`) (`self.Animal`) (`self.SurvivalEffect`))
    (set `/Game/Blueprints/GameMode/BP_AnimalCharacter.DisableMovement` false (`self.Animal`))
    (else
      (set `/Game/Blueprints/GameMode/BP_AnimalCharacter.DisableMovement` false (`self.Animal`)))))

(fn `CanInteract`
  (returns (Result :type Boolean))
  (bind _animal (`self.Animal`))
  ;[1 1 1] Unreal blueprint does not support the boolean circuit
  (`/Engine/EditorBlueprintResources/StandardMacros.IsValid` _animal
    (:`Is Valid`
      (return (and (>= (`self.WaterAmount`) 0.0) (`self.IsOverlapping`) (`/Game/Blueprints/GameMode/BP_AnimalCharacter.CatchPressed` _animal))))
    (:`Is Not Valid`
      (return false))))

(fn `UserConstructionScript`)