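; GI_AnimalData is a lookup store that holds animal data keyed by animal type.
; It wraps an AnimalData map with functions to add, check, get and clear entries.
; Get prints an error string when no entry exists for the requested type.
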(fn `Add`
  (params (AnimalType :type "/Game/Blueprints/Data/E_AnimalType Enum" :default "NewEnumerator0") (AnimalData :type "/Game/Blueprints/Data/AnimalData Structure"))
  (`BlueprintMapLibrary.Map_Add` (`self.AnimalData`) AnimalType AnimalData))

(fn `Clear`
  (`BlueprintMapLibrary.Map_Clear` (`self.AnimalData`)))

(fn `Get`
  (params (AnimalType :type "/Game/Blueprints/Data/E_AnimalType Enum" :default "NewEnumerator0"))
  (returns (AnimalData :type "/Game/Blueprints/Data/AnimalData Structure"))
  (bind (_value _returnvalue) (`BlueprintMapLibrary.Map_Find` (`self.AnimalData`) AnimalType))
  (if _returnvalue
    (return _value)
    (else
      (`KismetSystemLibrary.PrintString` "Failed to find animal data"))))

(fn `Has`
  (params (AnimalType :type "/Game/Blueprints/Data/E_AnimalType Enum" :default "NewEnumerator0"))
  (returns (Empty :type Boolean))
  (return (`BlueprintMapLibrary.Map_Contains` (`self.AnimalData`) AnimalType)))