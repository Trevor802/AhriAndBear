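; Procedural walkside Blueprint that builds a sidewalk of spline meshes along an editable spline in the Construction Script.
; It flattens spline points to Z=0, then splits each span into evenly sized sections near SectionLength, with shared offset, scale and height.
; Each span ends in a corner piece whose mesh or material depends on the next point's type and tangent size.
; The last span's corner piece wraps back toward the spline start.
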(fn `UserConstructionScript`
  (bind _spline (`self.Spline`))
  (bind _spline_2 (`self.Spline`))
  (bind _real_section_length (`self.Real Section Length`))
  (bind _spline_3 (`self.Spline`))
  (bind _spline_4 (`self.Spline`))
  (bind _spline_5 (`self.Spline`))
  (bind _spline_6 (`self.Spline`))
  (bind _currentdistance (`self.CurrentDistance`))
  (bind _currentdistance_2 (`self.CurrentDistance`))
  (bind _real_section_length_2 (`self.Real Section Length`))
  (bind _spline_7 (`self.Spline`))
  (bind _spline_8 (`self.Spline`))
  (bind _returnvalue (`KismetMathLibrary.MakeVector2D` (`self.Scale`) (`self.Height`)))
  (bind _returnvalue_2 (`KismetMathLibrary.MakeVector2D` (`self.Scale`) (`self.Height`)))
  (bind _returnvalue_3 (+ (`self.CurrentDistance`) (`self.Real Section Length`)))
  (bind _returnvalue_4 (+ (`self.CurrentDistance`) (`self.Real Section Length`)))
  (bind _returnvalue_5 (+ (`self.CurrentPoint`) 1))
  (bind _returnvalue_6 (`KismetMathLibrary.MakeVector2D` (- (`self.OffsetSpline`) 300.0)))
  (bind _returnvalue_7 (== (`SplineComponent.GetNumberOfSplinePoints` _spline_6) (+ (`self.CurrentPoint`) 1)))
  (bind _returnvalue_8 (`KismetMathLibrary.MakeVector2D` (- (`self.OffsetSpline`) 300.0)))
  (bind _returnvalue_9 (< (+ (`KismetMathLibrary.Abs` (.x (`SplineComponent.GetArriveTangentAtSplinePoint` _spline_4 _returnvalue_5 "Local"))) (`KismetMathLibrary.Abs` (.y (`SplineComponent.GetArriveTangentAtSplinePoint` _spline_4 _returnvalue_5 "Local")))) 1400.0))
  ;[0.8189 0.03898 0] Limit to Z=0
  (for _index (range (`SplineComponent.GetNumberOfSplinePoints` (`self.Spline`)))
    (`SplineComponent.SetLocationAtSplinePoint` _spline_3 _index (`KismetMathLibrary.MakeVector` (.x (`SplineComponent.GetLocationAtSplinePoint` _spline_3 _index "Local")) (.y (`SplineComponent.GetLocationAtSplinePoint` _spline_3 _index "Local"))) "Local" true))
  (set `self.CurrentPoint` 0)
  (set `self.CurrentDistance` 0.0)
  ;[1 0.465 0] Spline Road
  (for _index_2 (range (+ (`SplineComponent.GetNumberOfSplinePoints` (`self.Spline`)) 1))
    (bind _output_get (set `self.CurrentPoint` _index_2))
    (if (not (!= _output_get 0))
      (set `self.CurrentDistance` 300.0))
    (if (== (`SplineComponent.GetNumberOfSplinePoints` (`self.Spline`)) (`self.CurrentPoint`))
      (bind _returnvalue_10 (/ (- (`SplineComponent.GetSplineLength` _spline_8) (`SplineComponent.GetDistanceAlongSplineAtSplinePoint` _spline_8 _index_2)) (`self.SectionLength`)))
      (set `self.Real Section Length` _returnvalue_10)
      (set `self.NumberSections` (- (`KismetMathLibrary.FTrunc` _returnvalue_10) 2))
      (else
        (bind _returnvalue_11 (- (`SplineComponent.GetDistanceAlongSplineAtSplinePoint` _spline_7 (+ _index_2 1)) (`SplineComponent.GetDistanceAlongSplineAtSplinePoint` _spline_7 _index_2)))
        (bind _returnvalue_12 (`KismetMathLibrary.FTrunc` (/ _returnvalue_11 (`self.SectionLength`))))
        (set `self.Real Section Length` (/ _returnvalue_11 (`KismetMathLibrary.Conv_IntToDouble` _returnvalue_12)))
        (set `self.NumberSections` (- _returnvalue_12 2))))
    (for _index_3 (range (+ (`self.NumberSections`) 1))
      (set `self.locationFirstPoint` (`SplineComponent.GetLocationAtDistanceAlongSpline` _spline_5 _currentdistance_2 "Local"))
      (set `self.tangetFirstPoint` (`KismetMathLibrary.ClampVectorSize` (`SplineComponent.GetTangentAtDistanceAlongSpline` _spline_5 _currentdistance_2 "Local") 0.0 _real_section_length_2))
      (set `self.locationLastPoint` (`SplineComponent.GetLocationAtDistanceAlongSpline` _spline_5 _returnvalue_4 "Local"))
      (set `self.tangetLastPoint` (`KismetMathLibrary.ClampVectorSize` (`SplineComponent.GetTangentAtDistanceAlongSpline` _spline_5 _returnvalue_4 "Local") 0.0 _real_section_length_2))
      (if (not (and (== (`SplineComponent.GetNumberOfSplinePoints` (`self.Spline`)) (+ (`self.CurrentPoint`) 1)) (== _index_3 (+ (`self.NumberSections`) 1))))
        (bind _returnvalue_13 (`AddComponent|NODE_AddSplineMeshComponent-0` :`bManualAttachment` true))
        (`SplineMeshComponent.SetStartAndEnd` _returnvalue_13 (`self.locationFirstPoint`) (`self.tangetFirstPoint`) (`self.locationLastPoint`) (`self.tangetLastPoint`) true)
        (`SceneComponent.K2_AttachToComponent` _returnvalue_13 (`self.RoadSpline`) "None" "KeepRelative" "KeepRelative" "KeepRelative" true)
        (`PrimitiveComponent.SetCollisionEnabled` _returnvalue_13 "QueryAndPhysics")
        (`SplineMeshComponent.SetStartOffset` _returnvalue_13 _returnvalue_6 true)
        (`SplineMeshComponent.SetEndOffset` _returnvalue_13 _returnvalue_6 true)
        (`SplineMeshComponent.SetStartScale` _returnvalue_13 _returnvalue_2 true)
        (`SplineMeshComponent.SetEndScale` _returnvalue_13 _returnvalue_2 true)
        (set `self.CurrentDistance` (+ (`self.CurrentDistance`) (`self.Real Section Length`)))))
    ;[1 0.00337 0] Corner
    (set `self.locationFirstPoint` (`SplineComponent.GetLocationAtDistanceAlongSpline` _spline _currentdistance "Local"))
    (set `self.tangetFirstPoint` (`KismetMathLibrary.ClampVectorSize` (`SplineComponent.GetTangentAtDistanceAlongSpline` _spline _currentdistance "Local") 0.0 _real_section_length))
    (if (== (`SplineComponent.GetNumberOfSplinePoints` (`self.Spline`)) (+ (`self.CurrentPoint`) 1))
      (set `self.locationLastPoint` (`SplineComponent.GetLocationAtDistanceAlongSpline` _spline_2 300.0 "Local"))
      (set `self.tangetLastPoint` (`KismetMathLibrary.ClampVectorSize` (`SplineComponent.GetTangentAtDistanceAlongSpline` _spline_2 300.0 "Local") 0.0 (`self.SectionLength`)))
      (else
        (set `self.locationLastPoint` (`SplineComponent.GetLocationAtDistanceAlongSpline` _spline _returnvalue_3 "Local"))
        (set `self.tangetLastPoint` (`KismetMathLibrary.ClampVectorSize` (`SplineComponent.GetTangentAtDistanceAlongSpline` _spline _returnvalue_3 "Local") 0.0 _real_section_length))))
    (bind _returnvalue_14 (`AddComponent|NODE_AddSplineMeshComponent-1` :`bManualAttachment` true))
    (if (not (or (and (or (`|EnumEquality` (`SplineComponent.GetSplinePointType` _spline_4 _returnvalue_5) "Linear") _returnvalue_9) (not _returnvalue_7)) (and _returnvalue_7 (or _returnvalue_9 (`|EnumEquality` (`SplineComponent.GetSplinePointType` _spline_6 0) "Linear")))))
      (`StaticMeshComponent.SetStaticMesh` _returnvalue_14 "/Game/ProceduralBuildings/Geometry/Road/SM_walkside_6x6_corner.SM_walkside_6x6_corner")
      (else
        (`PrimitiveComponent.SetMaterial` _returnvalue_14 0 "/Game/ProceduralBuildings/Materials/Other/MI_walkside01_WA.MI_walkside01_WA")))
    (`SplineMeshComponent.SetStartAndEnd` _returnvalue_14 (`self.locationFirstPoint`) (`self.tangetFirstPoint`) (`self.locationLastPoint`) (`self.tangetLastPoint`) true)
    (`SceneComponent.K2_AttachToComponent` _returnvalue_14 (`self.RoadSpline`) "None" "KeepRelative" "KeepRelative" "KeepRelative" true)
    (`PrimitiveComponent.SetCollisionEnabled` _returnvalue_14 "QueryAndPhysics")
    (`SplineMeshComponent.SetStartOffset` _returnvalue_14 _returnvalue_8 true)
    (`SplineMeshComponent.SetEndOffset` _returnvalue_14 _returnvalue_8 true)
    (`SplineMeshComponent.SetStartScale` _returnvalue_14 _returnvalue true)
    (`SplineMeshComponent.SetEndScale` _returnvalue_14 _returnvalue true)
    (set `self.CurrentDistance` (+ (`self.CurrentDistance`) (`self.Real Section Length`)))))